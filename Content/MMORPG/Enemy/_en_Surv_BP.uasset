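; Melee enemy character Blueprint with a name and health bar widget that updates and turns toward the player's camera each tick.
; Attack passes a DoOnce that stops movement and plays one of two random montages; AttackEnded restores speed and re-arms it.
; Hand collisions toggled by events apply random damage, with DoOnce gates preventing repeat hits per swing.
; Incoming damage lowers health until death notifies the AnimBP, disables capsule collision and destroys the actor after a delay.
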(event `self.ReceiveBeginPlay`
  ;[1 1 1] Get widget reference
  (set `self.HPBarWidgetRef` (cast `/Game/MMORPG/Enemy/HPBarEnenmy` (`WidgetComponent.GetUserWidgetObject` (`self._hp_Bar`)) :!pure true))
  ;[1 1 1] Getting start speed
  (set `self.Start Max Speed` (`CharacterMovementComponent.MaxWalkSpeed` (`self.CharacterMovement`))))

(event `self.ReceiveTick`
  (params (DeltaSeconds :type "Float (single-precision)"))
  ;[1 1 1] Auto widget rotation to camera
  (`|ExecutionSequence`
    (:`then_0`
      ;[1 1 1] Draw hp to widget
      (`ProgressBar.SetPercent` (`/Game/MMORPG/Enemy/HPBarEnenmy._pb_HPBar` (`self.HPBarWidgetRef`)) (`KismetMathLibrary.NormalizeToRange` (`self.CurrentHP`) 0.0 (`self.MaxHP`)))
      ;[1 1 1] Draw name to widget
      (`TextBlock.SetText` (`/Game/MMORPG/Enemy/HPBarEnenmy._tb_mobname` (`self.HPBarWidgetRef`)) (`self.NPCName`)))
    (:`then_1`
      (`SceneComponent.K2_SetWorldRotation` (`self._hp_Bar`) (`KismetMathLibrary.FindLookAtRotation` (`SceneComponent.K2_GetComponentLocation` (`self._hp_Bar`)) (`SceneComponent.K2_GetComponentLocation` (`/Game/MMORPG/PlayerController/BP_ThirdPersonCharacter.FollowCamera` (cast `/Game/MMORPG/PlayerController/BP_ThirdPersonCharacter` (`GameplayStatics.GetPlayerCharacter` 0) :!pure true)))) false false))))

(event `Enable RightHand Collision`
  ;[1 1 1] Collsions
  (`PrimitiveComponent.SetCollisionEnabled` (`self.RightHand`) "QueryOnly")
  ;;[1 1 1] Sounds attack
  (`GameplayStatics.PlaySoundAtLocation` "/Game/MMORPG/CustomPlayerChatacter/Sounds/Audio/AttackAir.AttackAir" (0.0 0.0 0.0) (struct) 1.0 1.0 0.0 null null null null))

(event `AttackEnded`
  ;[1 1 1] Attack logic
  ;;[1 1 1] Restore monster speed
  (set `CharacterMovementComponent.MaxWalkSpeed` (`self.Start Max Speed`) (`self.CharacterMovement`))
  (goto _label :!via `Reset`))

(event `Disable RightHand Collision`
  ;[1 1 1] Collsions
  (`PrimitiveComponent.SetCollisionEnabled` (`self.RightHand`) "NoCollision")
  ;[1 1 1] Blocker multidamage
  (`self.Refresh right hand attack`))

(event `Attack`
  ;[1 1 1] Attack logic
  (if (not (`self.IsDead?`))
    (`/Engine/EditorBlueprintResources/StandardMacros.DoOnce` false :!label _label
      (:`Completed`
        ;;[1 1 1] Attack moment
        (set `CharacterMovementComponent.MaxWalkSpeed` 0.0 (`self.CharacterMovement`))
        ;;[1 1 1] Attack monester
        (if (`KismetMathLibrary.RandomBoolWithWeight` 0.5)
          (`self.PlayAnimMontage` "/Game/MMORPG/Enemy/Animations/_en_Surv_Attack1_Montage._en_Surv_Attack1_Montage")
          (else
            (`self.PlayAnimMontage` "/Game/MMORPG/Enemy/Animations/_en_Surv_Attack2_Montage._en_Surv_Attack2_Montage")))))))

(event `Enable LeftHand Collision`
  ;[1 1 1] Collsions
  (`PrimitiveComponent.SetCollisionEnabled` (`self.LeftHand`) "QueryOnly")
  ;;[1 1 1] Sounds attack
  (`GameplayStatics.PlaySoundAtLocation` "/Game/MMORPG/CustomPlayerChatacter/Sounds/Audio/AttackAir.AttackAir" (0.0 0.0 0.0) (struct) 1.0 1.0 0.0 null null null null))

(event `Disable LeftHand Collision`
  ;[1 1 1] Collsions
  (`PrimitiveComponent.SetCollisionEnabled` (`self.LeftHand`) "NoCollision")
  ;[1 1 1] Blocker multidamage
  (`self.Refresh left hand attack`))

(event `self.RightHand.OnComponentBeginOverlap`
  (params (OverlappedComponent :type "PrimitiveComponent Object Reference") (OtherActor :type "Actor Object Reference") (OtherComp :type "PrimitiveComponent Object Reference") (OtherBodyIndex :type Integer) (bFromSweep :type Boolean) (SweepResult :type "HitResult Structure (by ref)"))
  ;[1 1 1] Damage Register
  (if (!= OtherActor self)
    ;;[1 1 1] Multidamage checker
    (`/Engine/EditorBlueprintResources/StandardMacros.DoOnce` false :!label _label_2
      (:`Completed`
        (`GameplayStatics.ApplyDamage` OtherActor (`KismetMathLibrary.RandomFloatInRange` 5.0 10.0))
        (`GameplayStatics.PlaySoundAtLocation` "/Game/MMORPG/CustomPlayerChatacter/Sounds/Damage_Cue.Damage_Cue" (0.0 0.0 0.0) (struct) 1.0 1.0 0.0 null null null null :!label _label_3)))))

(event `Refresh right hand attack`
  ;[1 1 1] Damage Register
  (goto _label_2 :!via `Reset`))

(event `self.LeftHand.OnComponentBeginOverlap`
  (params (OverlappedComponent :type "PrimitiveComponent Object Reference") (OtherActor :type "Actor Object Reference") (OtherComp :type "PrimitiveComponent Object Reference") (OtherBodyIndex :type Integer) (bFromSweep :type Boolean) (SweepResult :type "HitResult Structure (by ref)"))
  ;[1 1 1] Damage Register
  (if (!= OtherActor self)
    ;;[1 1 1] Multidamage checker
    (`/Engine/EditorBlueprintResources/StandardMacros.DoOnce` false :!label _label_4
      (:`Completed`
        (`GameplayStatics.ApplyDamage` OtherActor (`KismetMathLibrary.RandomFloatInRange` 5.0 10.0))
        (goto _label_3)))))

(event `Refresh left hand attack`
  ;[1 1 1] Damage Register
  (goto _label_4 :!via `Reset`))

(event `self.ReceiveAnyDamage`
  (params (Damage :type "Float (single-precision)") (DamageType :type "DamageType Object Reference") (InstigatedBy :type "Controller Object Reference") (DamageCauser :type "Actor Object Reference"))
  ;[1 1 1] Damage given
  (if (not (`self.IsDead?`))
    (bind _output_get (set `self.CurrentHP` (`KismetMathLibrary.SelectFloat` 0.0 (- (`self.CurrentHP`) Damage) (>= Damage (`self.CurrentHP`)))))
    (`|ExecutionSequence`
      (:`then_0`
        (if (`KismetMathLibrary.RandomBoolWithWeight` 0.8)
          (`GameplayStatics.PlaySoundAtLocation` "/Game/MMORPG/CustomPlayerChatacter/Sounds/Damage.Damage" (`self.K2_GetActorLocation` self) (struct) 1.0 1.0 0.0 null null null null)))
      (:`then_1`
        ;;[1 1 1] Mob death
        (if (<= _output_get 0.0)
          (`self.Death`)
          (`KismetSystemLibrary.PrintString` (`KismetStringLibrary.Concat_StrStr` (`KismetTextLibrary.Conv_TextToString` (`self.NPCName`)) " is Death") true true (struct :`A` 1.0)))))))

(event `Death`
  (set `self.IsDead?` true)
  (`/Game/MMORPG/Enemy/Animations/_en_Surv_AnimBP.DeathOnAnimBP` (cast `/Game/MMORPG/Enemy/Animations/_en_Surv_AnimBP` (`SkeletalMeshComponent.GetAnimInstance` (`self.Mesh`)) :!pure true))
  (`self.StopAnimMontage` "/Game/MMORPG/Enemy/Animations/_en_Surv_Attack1_Montage._en_Surv_Attack1_Montage")
  (`self.StopAnimMontage` "/Game/MMORPG/Enemy/Animations/_en_Surv_Attack2_Montage._en_Surv_Attack2_Montage")
  (`PrimitiveComponent.SetCollisionEnabled` (`self.CapsuleComponent`) "NoCollision")
  (`GameplayStatics.PlaySoundAtLocation` "/Game/MMORPG/Audio/DeathSound.DeathSound" (`self.K2_GetActorLocation` self) (struct) 1.0 1.0 0.0 null null null null)
  (`KismetSystemLibrary.Delay` 10.0)
  (`self.K2_DestroyActor`))

(fn `UserConstructionScript`)