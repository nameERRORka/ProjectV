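; Zombie enemy character for an MMORPG, with melee attacks, a floating health bar, death and an XP reward.
; Attack halts movement and plays one of two random montages until AttackEnded restores speed.
; Per-hand collision events open hit windows, with DoOnce gates blocking repeat damage.
; Tick updates and turns the name/HP widget toward the player camera; death disables capsule collision, grants last attacker random XP and destroys the actor after a delay.
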(event `self.ReceiveBeginPlay`
  ;[1 1 1] Get widget reference
  (set `self.HPBarWidgetRef` (cast `/Game/MMORPG/Enemy/UI/HPBarEnenmy` (`WidgetComponent.GetUserWidgetObject` (`self._hp_Bar`)) :!pure true))
  (set `self.Max start speed` (`CharacterMovementComponent.MaxWalkSpeed` (`self.CharacterMovement`))))

(event `self.ReceiveTick`
  (params (DeltaSeconds :type "Float (single-precision)"))
  ;[1 1 1] Auto widget rotation to camera
  (`|ExecutionSequence`
    (:`then_0`
      ;[1 1 1] Draw hp to widget
      (`ProgressBar.SetPercent` (`/Game/MMORPG/Enemy/UI/HPBarEnenmy._pb_HPBar` (`self.HPBarWidgetRef`)) (`KismetMathLibrary.NormalizeToRange` (`self.CurrentHP`) 0.0 (`self.MaxHP`)))
      ;[1 1 1] Draw name to widget
      (`TextBlock.SetText` (`/Game/MMORPG/Enemy/UI/HPBarEnenmy._tb_mobname` (`self.HPBarWidgetRef`)) (`self.NPCName`)))
    (:`then_1`
      (`SceneComponent.K2_SetWorldRotation` (`self._hp_Bar`) (`KismetMathLibrary.FindLookAtRotation` (`SceneComponent.K2_GetComponentLocation` (`self._hp_Bar`)) (`SceneComponent.K2_GetComponentLocation` (`/Game/MMORPG/PlayerController/BP_ThirdPersonCharacter.FollowCamera` (cast `/Game/MMORPG/PlayerController/BP_ThirdPersonCharacter` (`GameplayStatics.GetPlayerCharacter` 0) :!pure true)))) false false))))

(event `Attack`
  ;[1 0.5573 0.5573] Attack
  (if (not (`self.IsDead?`))
    (`/Engine/EditorBlueprintResources/StandardMacros.DoOnce` false :!label _label
      (:`Completed`
        ;;[1 1 1] Attack Moment
        (set `CharacterMovementComponent.MaxWalkSpeed` 0.0 (`self.CharacterMovement`))
        (if (`KismetMathLibrary.RandomBoolWithWeight` 0.5)
          ;;[1 1 1] Left hand attack
          (`self.PlayAnimMontage` "/Game/MMORPG/Enemy/Animations/_en_Surv_Attack1_Montage._en_Surv_Attack1_Montage")
          (else
            ;;[1 1 1] Double attack
            (`self.PlayAnimMontage` "/Game/MMORPG/Enemy/Animations/_en_Surv_Attack2_Montage._en_Surv_Attack2_Montage")))))))

(event `AttackEnded`
  ;[1 0.5573 0.5573] Attack
  (set `CharacterMovementComponent.MaxWalkSpeed` (`self.Max start speed`) (`self.CharacterMovement`))
  (goto _label :!via `Reset`))

(event `Enable right hand collision`
  ;[1 1 1] Collision controller right hand
  (`PrimitiveComponent.SetCollisionEnabled` (`self.RightHand`) "QueryOnly")
  (`GameplayStatics.PlaySoundAtLocation` "/Game/MMORPG/CustomPlayerChatacter/Sounds/Audio/AttackAir2.AttackAir2" (`SceneComponent.GetSocketLocation` (`self.RightHand`) "None") (struct) 1.0 1.0 0.0 null null null null))

(event `Refresh right attack`
  ;[1 1 1] Damage register
  ;;[1 1 1] Double damage blocker
  (goto _label_2 :!via `Reset`))

(event `Disable right hand collision`
  ;[1 1 1] Collision controller right hand
  (`PrimitiveComponent.SetCollisionEnabled` (`self.RightHand`) "NoCollision")
  ;[1 1 1] Overlap controller
  (`self.Refresh right attack`))

(event `self.RightHand.OnComponentBeginOverlap`
  (params (OverlappedComponent :type "PrimitiveComponent Object Reference") (OtherActor :type "Actor Object Reference") (OtherComp :type "PrimitiveComponent Object Reference") (OtherBodyIndex :type Integer) (bFromSweep :type Boolean) (SweepResult :type "HitResult Structure (by ref)"))
  ;[1 1 1] Damage register
  (if (!= OtherActor self)
    ;;[1 1 1] Double damage blocker
    (`/Engine/EditorBlueprintResources/StandardMacros.DoOnce` false :!label _label_2
      (:`Completed`
        (`GameplayStatics.ApplyDamage` OtherActor (`KismetMathLibrary.RandomFloatInRange` 2.0 5.0))
        (`GameplayStatics.PlaySoundAtLocation` "/Game/MMORPG/Audio/Hit/Hit.Hit" (0.0 0.0 0.0) (struct) 1.0 1.0 0.0 null null null null)))))

(event `Enable left hand collision`
  ;[1 1 1] Collision controller left hand controller
  (`PrimitiveComponent.SetCollisionEnabled` (`self.LeftHand`) "QueryOnly")
  (`GameplayStatics.PlaySoundAtLocation` "/Game/MMORPG/CustomPlayerChatacter/Sounds/Audio/AttackAir2.AttackAir2" (`SceneComponent.GetSocketLocation` (`self.LeftHand`) "None") (struct) 1.0 1.0 0.0 null null null null))

(event `Refresh left attack`
  ;[1 1 1] Damage register
  ;;[1 1 1] Double damage blocker
  (goto _label_3 :!via `Reset`))

(event `self.LeftHand.OnComponentBeginOverlap`
  (params (OverlappedComponent :type "PrimitiveComponent Object Reference") (OtherActor :type "Actor Object Reference") (OtherComp :type "PrimitiveComponent Object Reference") (OtherBodyIndex :type Integer) (bFromSweep :type Boolean) (SweepResult :type "HitResult Structure (by ref)"))
  ;[1 1 1] Damage register
  (if (!= OtherActor self)
    ;;[1 1 1] Double damage blocker
    (`/Engine/EditorBlueprintResources/StandardMacros.DoOnce` false :!label _label_3
      (:`Completed`
        (`GameplayStatics.ApplyDamage` OtherActor (`KismetMathLibrary.RandomFloatInRange` 2.0 5.0))
        (`GameplayStatics.PlaySoundAtLocation` "/Game/MMORPG/Audio/Hit/Hit.Hit" (0.0 0.0 0.0) (struct) 1.0 1.0 0.0 null null null null)))))

(event `Disable left hand collision`
  ;[1 1 1] Collision controller left hand controller
  (`PrimitiveComponent.SetCollisionEnabled` (`self.LeftHand`) "NoCollision")
  ;[1 1 1] Overlap controller
  (`self.Refresh left attack`))

(event `self.ReceiveAnyDamage`
  (params (Damage :type "Float (single-precision)") (DamageType :type "DamageType Object Reference") (InstigatedBy :type "Controller Object Reference") (DamageCauser :type "Actor Object Reference"))
  ;[1 1 1] Damage getter
  (set `self.LastHitActor` DamageCauser)
  (if (not (`self.IsDead?`))
    (bind _output_get (set `self.CurrentHP` (`KismetMathLibrary.SelectFloat` 0.0 (- (`self.CurrentHP`) Damage) (>= Damage (`self.CurrentHP`)))))
    (`|ExecutionSequence`
      (:`then_0`
        (if (`KismetMathLibrary.RandomBoolWithWeight` 0.8)
          (`GameplayStatics.PlaySoundAtLocation` "/Game/MMORPG/CustomPlayerChatacter/Sounds/Damage.Damage" (`SceneComponent.K2_GetComponentLocation` (`self.Mesh`)) (struct) 1.0 1.0 0.0 null null null null)))
      (:`then_1`
        (if (<= _output_get 0.0)
          (`self.Death`)
          (`KismetSystemLibrary.PrintString` (`KismetStringLibrary.Concat_StrStr` (`KismetTextLibrary.Conv_TextToString` (`self.NPCName`)) " is dead!")))))))

(event `Death`
  (set `self.IsDead?` true)
  (`/Game/MMORPG/Enemy/Animations/_en_Surv_AnimBP.Death on AnimBP` (cast `/Game/MMORPG/Enemy/Animations/_en_Surv_AnimBP` (`SkeletalMeshComponent.GetAnimInstance` (`self.Mesh`)) :!pure true))
  (`self.StopAnimMontage` "/Game/MMORPG/Enemy/Animations/_en_Surv_Attack1_Montage._en_Surv_Attack1_Montage")
  (`self.StopAnimMontage` "/Game/MMORPG/Enemy/Animations/_en_Surv_Attack2_Montage._en_Surv_Attack2_Montage")
  (`PrimitiveComponent.SetCollisionEnabled` (`self.CapsuleComponent`) "NoCollision")
  (`GameplayStatics.PlaySoundAtLocation` "/Game/MMORPG/CustomPlayerChatacter/Sounds/Death_Cue.Death_Cue" (0.0 0.0 0.0) (struct) 1.0 1.0 0.0 null null null null)
  (`|ExecutionSequence`
    (:`then_0`
      (`KismetSystemLibrary.Delay` 20.0)
      (`self.K2_DestroyActor`))
    (:`then_1`
      ;[1 1 1] Level up for player
      (`/Game/MMORPG/PlayerController/LVLStatsComponent/LevelStats.Take EXP from mob` (`/Game/MMORPG/PlayerController/BP_ThirdPersonCharacter.LevelStats` (cast `/Game/MMORPG/PlayerController/BP_ThirdPersonCharacter` (`self.LastHitActor`) :!pure true)) (`KismetMathLibrary.RandomIntegerInRange` 200 500)))))

(fn `UserConstructionScript`)