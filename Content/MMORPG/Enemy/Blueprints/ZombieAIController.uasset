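; AI controller for the zombie enemy that switches between attacking the player and wandering.
; After a short startup delay it caches the zombie and its spawn point, then Tick runs a macro checking player 0's distance and death state.
; A living player in range is chased and attacked; otherwise the zombie patrols random navigable points around spawn with pauses.
; DoOnce gates prevent repeated move orders, and movement stops when the zombie dies.
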(event `self.ReceiveBeginPlay`
  ;[1 1 1] Preloader
  (`KismetSystemLibrary.Delay` 0.2)
  (set `self.ZombieRef` (cast `/Game/MMORPG/Enemy/Blueprints/Zombie_BP` (`self.K2_GetPawn`) :!pure true))
  (set `self.SpawnLocation` (`self.K2_GetActorLocation` (cast `/Game/MMORPG/Enemy/Blueprints/Zombie_BP` (`self.K2_GetPawn`) :!pure true)))
  (set `self.PreLoad` true))

(event `self.ReceiveTick`
  (params (DeltaSeconds :type "Float (single-precision)"))
  (if (`self.PreLoad`)
    ;[1 1 1] Is dead blocker
    (if (not (`/Game/MMORPG/Enemy/Blueprints/Zombie_BP.IsDead?` (`self.ZombieRef`)))
      (`self.AISearcherEnemy` 500.0
        (:`IsAliveEnemy`
          ;[1 0.526 0.526] Attack player
          (`/Engine/EditorBlueprintResources/StandardMacros.DoOnce` false :!label _label
            (:`Completed`
              (`|AIMoveTo` (`self.ZombieRef`) (0.0 0.0 0.0) (`GameplayStatics.GetPlayerCharacter` 0) 50.0
                (:`OnSuccess`
                  (`/Game/MMORPG/Enemy/Blueprints/Zombie_BP.Attack` (`self.ZombieRef`))
                  (goto _label :!via `Reset`))
                (:`OnFail`
                  (goto _label :!via `Reset`))))))
        (:`IsDeadEnemy`
          _)
        (:`Rest`
          _))
      ;[1 1 1] Patrolling
      (`/Engine/EditorBlueprintResources/StandardMacros.DoOnce` false :!label _label_2
        (:`Completed`
          (`|AIMoveTo` (`self.ZombieRef`) (`NavigationSystemV1.K2_GetRandomLocationInNavigableRadius` (`self.SpawnLocation`) 1000.0 null null) null
            (:`OnSuccess`
              _)
            (:`OnFail`
              _))
          (`KismetSystemLibrary.Delay` 10.0)
          (goto _label_2 :!via `Reset`)))
      (else
        (`/Engine/EditorBlueprintResources/StandardMacros.DoOnce` false
          (:`Completed`
            (`self.StopMovement`)))))))

(fn `UserConstructionScript`)